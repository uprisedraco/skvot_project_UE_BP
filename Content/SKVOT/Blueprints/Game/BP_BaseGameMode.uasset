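; Base game mode that polls for a time-based game fail condition.
; On BeginPlay it starts a looping one-second timer that checks whether game time has reached the total WavesDuration.
; When that condition is met it only clears the timer, with no further fail handling in this graph.
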(event Custom|CheckGameFailCondition
  (if (CallFunction|CheckFailbyTimeCondition)
    (Utilities|Time|ClearandInvalidateTimerbyHandle (Variables|Default|GetGameFailTimer))))

(event EventBeginPlay
  (bind _returnvalue (Utilities|Time|SetTimerbyEvent (delegate Custom|CheckGameFailCondition) 1.0 true))
  (Variables|Default|SetGameFailTimer _returnvalue))

(fn ConstructionScript)

(fn CheckFailbyTimeCondition
  (return (>= (Utilities|Time|GetGameTimeinSeconds) (Math|Timespan|GetTotalSeconds (Variables|Default|GetWavesDuration)))))