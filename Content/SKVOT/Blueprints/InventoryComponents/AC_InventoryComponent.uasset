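; Inventory component that stores items as stacks in a slot array sized on BeginPlay.
; AddItemToInventory moves one unit per call into a matching stack below its DT_ItemData limit, else into an empty slot, setting IsFull when none remains.
; AddToStack writes at the quantity as index, not the found slot.
; TransferSlot merges matching stacks with overflow left at source, or swaps differing slots, then fires both inventories' update events.
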(event Custom|UpdateInventory
  (Default|CallOnInventoryUpdated))

(event EventBeginPlay
  (Utilities|Array|Resize (Variables|Default|GetItems) (Variables|Default|GetInventorySize)))

(fn AddItemtoInventory
  (params (Item :type BP%20Interactable%20Item%20Object%20Reference))
  (bind (_slotavailable _index) (CallFunction|AnySlotAvailable))
  (bind _output_get (LocalVariables|SetItemData (Actor|GetComponentbyClass Item "/Game/SKVOT/AC_ItemData.AC_ItemData_C")))
  (while (and (> (Variables|/Game/SKVOT/AC_ItemData.AC_ItemData_C|GetItemQuantity _output_get) 0) (not (LocalVariables|GetIsFull)))
    (bind (_array_index _slotavailable_2) (CallFunction|FindSlot (.rowname (Variables|/Game/SKVOT/AC_ItemData.AC_ItemData_C|GetItemId (LocalVariables|GetItemData)))))
    (if _slotavailable_2
      (CallFunction|AddtoStack _array_index 1)
      (Math|Integer|DecrementInt (Variables|/Game/SKVOT/AC_ItemData.AC_ItemData_C|GetItemQuantity (LocalVariables|GetItemData))
        (:%20%20
          (return true 0)))
      (elif _slotavailable
        (CallFunction|CreateNewStack (.rowname (Variables|/Game/SKVOT/AC_ItemData.AC_ItemData_C|GetItemId (LocalVariables|GetItemData))) 1 _index)
        (Math|Integer|DecrementInt (Variables|/Game/SKVOT/AC_ItemData.AC_ItemData_C|GetItemQuantity (LocalVariables|GetItemData))
          (:%20%20
            (return true 0)))
        (else
          (LocalVariables|SetIsFull true)))))
  (return (not (LocalVariables|GetIsFull)) (Variables|/Game/SKVOT/AC_ItemData.AC_ItemData_C|GetItemQuantity (LocalVariables|GetItemData))))

(fn FindSlot
  (params (ItemId :type Name))
  (for (_array_element _array_index) (Variables|Default|GetItems)
    (if (and (== ItemId (.ItemID (Utilities|Struct|BreakS_ItemSlot _array_element))) (< (.ItemQuantity (Utilities|Struct|BreakS_ItemSlot _array_element)) (CallFunction|GetMaxStackSize ItemId)))
      (return _array_index true)))
  (return -1 false))

(fn GetMaxStackSize
  (params (ItemID :type Name))
  (bind _returnvalue (Utilities|GetDataTableRow "/Game/SKVOT/DT_ItemData.DT_ItemData" ItemID)
    (:then
      (return (Utilities|Struct|BreakS_ItemData _returnvalue)))))

(fn AddtoStack
  (params (Index :type Integer) (ItemQuantity :type Integer))
  (bind _items (Variables|Default|GetItems))
  (bind _output (Utilities|Array|Get(acopy) _items Index))
  (Utilities|Array|SetArrayElem (Variables|Default|GetItems) ItemQuantity (Utilities|Struct|MakeS_ItemSlot (.itemid _output) (+ (.itemquantity _output) ItemQuantity))))

(fn AnySlotAvailable
  (for (_array_element _array_index) (Variables|Default|GetItems)
    (if (== (.ItemQuantity (Utilities|Struct|BreakS_ItemSlot _array_element)) 0)
      (return true _array_index)))
  (return false -1))

(fn CreateNewStack
  (params (ItemId :type Name) (ItemQuantity :type Integer) (Index :type Integer))
  (Utilities|Array|SetArrayElem (Variables|Default|GetItems) Index (Utilities|Struct|MakeS_ItemSlot ItemId ItemQuantity)))

(fn TransferSlot
  (params (Index :type Integer) (SourceIndex :type Integer) (SourceInventory :type AC%20Inventory%20Component%20Object%20Reference))
  (bind _items (Variables|Default|GetItems))
  (bind _output (Utilities|Array|Get(acopy) _items Index))
  (Utilities|FlowControl|Sequence
    (:then_0
      (LocalVariables|SetSourceSlot (Utilities|Array|Get(acopy) (Variables|AC_InventoryComponent_C|GetItems SourceInventory) SourceIndex))
      (if (== (.ItemID (Utilities|Struct|BreakS_ItemSlot (LocalVariables|GetSourceSlot))) (.ItemID (Utilities|Struct|BreakS_ItemSlot (Utilities|Array|Get(acopy) (Variables|Default|GetItems) Index))))
        (CallFunction|CreateNewStack SourceInventory (select (> (Math|Integer|Clamp(Integer) (- (+ (.ItemQuantity (Utilities|Struct|BreakS_ItemSlot (LocalVariables|GetSourceSlot))) (.ItemQuantity (Utilities|Struct|BreakS_ItemSlot (Utilities|Array|Get(acopy) (Variables|Default|GetItems) Index)))) (CallFunction|GetMaxStackSize (.ItemID (Utilities|Struct|BreakS_ItemSlot (LocalVariables|GetSourceSlot))))) 0 (CallFunction|GetMaxStackSize (.ItemID (Utilities|Struct|BreakS_ItemSlot (LocalVariables|GetSourceSlot))))) 0) (.ItemID (Utilities|Struct|BreakS_ItemSlot (LocalVariables|GetSourceSlot))) "None") (Math|Integer|Clamp(Integer) (- (+ (.ItemQuantity (Utilities|Struct|BreakS_ItemSlot (LocalVariables|GetSourceSlot))) (.ItemQuantity (Utilities|Struct|BreakS_ItemSlot (Utilities|Array|Get(acopy) (Variables|Default|GetItems) Index)))) (CallFunction|GetMaxStackSize (.ItemID (Utilities|Struct|BreakS_ItemSlot (LocalVariables|GetSourceSlot))))) 0 (CallFunction|GetMaxStackSize (.ItemID (Utilities|Struct|BreakS_ItemSlot (LocalVariables|GetSourceSlot))))) SourceIndex)
        (CallFunction|CreateNewStack (Utilities|Struct|BreakS_ItemSlot (LocalVariables|GetSourceSlot)) (Math|Integer|Clamp(Integer) (+ (.ItemQuantity (Utilities|Struct|BreakS_ItemSlot (LocalVariables|GetSourceSlot))) (.ItemQuantity (Utilities|Struct|BreakS_ItemSlot (Utilities|Array|Get(acopy) (Variables|Default|GetItems) Index)))) 0 (CallFunction|GetMaxStackSize (.ItemID (Utilities|Struct|BreakS_ItemSlot (LocalVariables|GetSourceSlot))))) Index)
        (else
          (CallFunction|CreateNewStack SourceInventory (.itemid _output) (.itemquantity _output) SourceIndex)
          (CallFunction|CreateNewStack (.ItemID (Utilities|Struct|BreakS_ItemSlot (LocalVariables|GetSourceSlot))) (.ItemQuantity (Utilities|Struct|BreakS_ItemSlot (LocalVariables|GetSourceSlot))) Index))))
    (:then_1
      (CallFunction|UpdateInventory)
      (CallFunction|UpdateInventory SourceInventory))))