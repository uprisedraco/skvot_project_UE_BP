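; BP_Chest is an interactable storage container that holds items in its own inventory component.
; On BeginPlay it resizes the component's Items array to ContainerSize.
; On interaction it casts the instigator to BP_ThirdPersonCharacter and has that character create a container display for the chest's inventory, leaving the UI to the character.
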(event EventBeginPlay
  (Utilities|Array|Resize (Variables|/Game/SKVOT/Blueprints/InventoryComponents/AC_InventoryComponent.AC_InventoryComponent_C|GetItems (Variables|Default|GetAC_InventoryComponent)) (Variables|Default|GetContainerSize)))

(fn ConstructionScript
  (|CallParentFunction))

(fn InteractwithItem
  (bind _asbp_third_person_character (Utilities|Casting|CastToBP_ThirdPersonCharacter (Variables|Default|GetInteractInstigator)))
  (Default|CreateContainerDisplay _asbp_third_person_character (Variables|Default|GetAC_InventoryComponent)))