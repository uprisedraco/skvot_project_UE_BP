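; Base interactable item actor that players can add to their inventory.
; Box collider overlaps, handled only on the server, tell instigators implementing BPI_Interact which item is in range, passing none on exit.
; InteractWithItem adds the item to the stored instigator's AC_InventoryComponent and destroys the actor once added.
; The Server AddItemToInventory RPC is an empty stub.
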(event OnComponentBeginOverlap(BoxCollider)
  (params (OverlappedComponent :type Primitive%20Component%20Object%20Reference) (OtherActor :type Actor%20Object%20Reference) (OtherComp :type Primitive%20Component%20Object%20Reference) (OtherBodyIndex :type Integer) (bFromSweep :type Boolean) (SweepResult :type Hit%20Result%20Structure%20%28by%20ref%29))
  (Networking|SwitchHasAuthority
    (:Authority
      (CallFunction|OverlapwithPlayer OtherActor self))))

(event OnComponentEndOverlap(BoxCollider)
  (params (OverlappedComponent :type Primitive%20Component%20Object%20Reference) (OtherActor :type Actor%20Object%20Reference) (OtherComp :type Primitive%20Component%20Object%20Reference) (OtherBodyIndex :type Integer))
  (Networking|SwitchHasAuthority
    (:Authority
      (CallFunction|OverlapwithPlayer OtherActor))))

(event Custom|Server%20|%20AddItemToInventory)

(fn ConstructionScript)

(fn OverlapwithPlayer
  (params (InteractInstigator :type Actor%20Object%20Reference) (Item :type BP%20Interactable%20Item%20Object%20Reference))
  (if (Utilities|DoesObjectImplementInterface InteractInstigator "/Game/SKVOT/Blueprints/Interfaces/BPI_Interact.BPI_Interact_C")
    (bind _output_get (Variables|Default|SetInteractInstigator InteractInstigator))
    (Class|BPIInteract|InteractwithItem(Message) _output_get Item)))

(fn InteractwithItem
  (bind _interactinstigator (Variables|Default|GetInteractInstigator))
  (bind _returnvalue (Actor|GetComponentbyClass _interactinstigator "/Game/SKVOT/Blueprints/ActorComponents/AC_InventoryComponent.AC_InventoryComponent_C"))
  (Utilities|IsValid _returnvalue
    (:Is%20Valid
      (bind _isadded (Default|AddItemtoInventory _returnvalue self))
      (if _isadded
        (Actor|DestroyActor self)))))