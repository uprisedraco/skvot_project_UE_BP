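; BP_BasicRevolver is a revolver weapon item whose attack traces a shot and plays a gunfire effect.
; Attack uses a two-step trace: from the owner's TP_Camera-tagged camera to find the aim point, then from the Muzzle socket toward it.
; Both traces draw debug lines, the second hit result is unused, and NE_Gunfire spawns at the muzzle.
; EnableCollisionAndDisableInteract only turns off the box collider's collision.
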(fn ConstructionScript
  (|CallParentFunction))

(fn Attack
  (bind _returnvalue (Components|GetOwner))
  (bind _returnvalue_2 (Actor|GetComponentsbyTag _returnvalue "/Script/Engine.CameraComponent" "TP_Camera"))
  (bind _output (Utilities|Array|Get(acopy) _returnvalue_2))
  (bind _returnvalue_3 (Transformation|GetWorldLocation _output))
  (bind _outhit (Collision|LineTraceByChannel _returnvalue_3 (+ _returnvalue_3 (* (Math|Vector|GetForwardVector _output) (Variables|Default|GetDistance))) "TraceTypeQuery3" false (Utilities|Array|MakeArray self (Components|GetOwner)) "ForDuration"))
  (Collision|LineTraceByChannel (Transformation|GetSocketLocation (Variables|Default|GetStaticMesh) "Muzzle") (select (.bBlockingHit (Collision|BreakHitResult _outhit)) (.Location (Collision|BreakHitResult _outhit)) (.TraceEnd (Collision|BreakHitResult _outhit))) "TraceTypeQuery3" false (Utilities|Array|MakeArray self (Components|GetOwner)) "ForDuration" true "(R=0.083333,G=0.000000,B=1.000000,A=1.000000)" "(R=1.000000,G=0.750000,B=0.000000,A=1.000000)")
  (Niagara|SpawnSystematLocation "/Game/SKVOT/VFX/Explosion/NE_Gunfire.NE_Gunfire" (Transformation|GetSocketLocation (Variables|Default|GetStaticMesh) "Muzzle")))

(fn EnableCollisionandDisableInteract
  (Collision|SetCollisionEnabled (Variables|Default|GetBoxCollider) "NoCollision"))