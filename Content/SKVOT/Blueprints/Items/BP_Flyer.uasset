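; BP_Flyer is an interactable item whose mesh rises when the player interacts with it.
; It extends a parent item class, calling each parent handler before swapping its text render to the interaction prompt on player overlap.
; Interacting hides the text, lifts the body mesh and sets IsInteracted.
; Ending overlap restores the default visible text and, if that flag is set, lowers the mesh and clears it.
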(fn ConstructionScript
  (|CallParentFunction))

(fn InteractwithItem
  (|CallParentFunction)
  (Rendering|SetVisibility (Variables|Default|GetTextRender) false false)
  (Transformation|AddRelativeLocation (Variables|Default|GetBodyMesh) "0.000000,0.000000,60.000000" false false)
  (Variables|Default|SetIsInteracted true))

(fn OverlapwithPlayer
  (|CallParentFunction)
  (Rendering|Components|TextRender|SetText (Variables|Default|GetTextRender) (LocalVariables|GetInteractionText)))

(fn EndOverlapwithPlayer
  (|CallParentFunction)
  (Rendering|Components|TextRender|SetText (Variables|Default|GetTextRender) (LocalVariables|GetDefaultItemText))
  (Rendering|SetVisibility (Variables|Default|GetTextRender) true false)
  (if (Variables|Default|GetIsInteracted)
    (Transformation|AddRelativeLocation (Variables|Default|GetBodyMesh) "0.000000,0.000000,-60.000000" false false)
    (Variables|Default|SetIsInteracted false)))