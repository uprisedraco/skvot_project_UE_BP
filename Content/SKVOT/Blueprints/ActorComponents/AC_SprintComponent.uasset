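; Actor component that adds a networked toggle between walking and running to its owner.
; The run toggle input calls a server event that flips IsRunning and sets CurrentSpeed to the run or walk speed.
; A RepNotify on CurrentSpeed applies the value to MaxWalkSpeed on the owner's CharacterMovementComponent, so the speed change follows replication.
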(event Input|EnhancedActionEvents|EnhancedInputActionIA_RunToggle
  (params (ActionValue :type Boolean) (ElapsedSeconds :type Float%20%28double-precision%29) (TriggeredSeconds :type Float%20%28double-precision%29) (InputAction :type Input%20Action%20Object%20Reference :default "/Game/SKVOT/Inputs/Actions/IA_RunToggle.IA_RunToggle"))
  (CallFunction|Server|EnableSprint))

(event Custom|Server%20|%20EnableSprint
  (CallFunction|EnableSprint (not (Variables|Default|GetIsRunning))))

(fn EnableSprint
  (params (Enable :type Boolean))
  (if (not (== Enable (Variables|Default|GetIsRunning)))
    (Variables|Default|SetCurrentSpeed (Math|Float|SelectFloat (Variables|Default|GetRunSpeed) (Variables|Default|GetWalkSpeed) Enable))
    (Variables|Default|SetIsRunning Enable)))

(fn OnRepCurrentSpeed
  (bind _returnvalue (Components|GetOwner))
  (bind _returnvalue_2 (Actor|GetComponentbyClass _returnvalue "/Script/Engine.CharacterMovementComponent"))
  (Utilities|IsValid _returnvalue_2
    (:Is%20Valid
      (Variables|/Script/Engine.CharacterMovementComponent|SetMaxWalkSpeed _returnvalue_2 (Variables|Default|GetCurrentSpeed)))))