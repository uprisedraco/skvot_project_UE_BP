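; Actor component that manages which ability components its owning actor has, granting a configured set of initial abilities when play begins on the authority.
; Each ability is a component class that AddAbility instantiates on the owner and records in RegisteredAbilities, skipping any already registered.
; RemoveAbility destroys the owner's component of that class and unregisters it, while HasAbility checks the registered list.
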(event EventBeginPlay
  (Networking|SwitchHasAuthority
    (:Authority
      (for _array_element (Variables|Default|GetInitialAbilities)
        (CallFunction|AddAbility _array_element)))))

(fn AddAbility
  (params (NewAbility :type Actor%20Component%20Class%20Reference))
  (if (not (CallFunction|HasAbility NewAbility))
    (Game|AddComponentbyClass (Components|GetOwner) NewAbility)
    (Utilities|Array|Add (Variables|Default|GetRegisteredAbilities) NewAbility)))

(fn RemoveAbility
  (params (Ability :type Actor%20Component%20Class%20Reference))
  (Components|DestroyComponent (Actor|GetComponentbyClass (Components|GetOwner) Ability))
  (Utilities|Array|RemoveItem (Variables|Default|GetRegisteredAbilities) Ability))

(fn HasAbility
  (params (Ability :type Actor%20Component%20Class%20Reference))
  (return (Utilities|Array|ContainsItem (Variables|Default|GetRegisteredAbilities) Ability)))