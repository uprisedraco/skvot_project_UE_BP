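; AC_HealthComponent is an actor component that tracks an actor's health and handles its death.
; ChangeHealthByAmoun subtracts the given amount from CurrentHealth and clamps the result between zero and MaxHealth.
; When IsOutOfHealth finds health at zero, it calls CallDead and then destroys the component.
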(fn ChangeHealthbyAmoun
  (params (HealthAmount :type Float%20%28double-precision%29))
  (Variables|Default|SetCurrentHealth (Math|Float|Clamp(Float) (- (Variables|Default|GetCurrentHealth) HealthAmount) 0.0 (Variables|Default|GetMaxHealth)))
  (if (CallFunction|IsOutOfHealth)
    (Default|CallDead)
    (Components|DestroyComponent)))

(fn IsOutOfHealth
  (return (<= (Variables|Default|GetCurrentHealth) 0.0)))