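; Inventory component that holds items in a fixed-size slot array and equips a revolver from the first slot on weapon-slot input.
; AddItemToInventory moves one unit per call, seeking a non-full matching stack via DT_ItemData limits, then an empty slot.
; TransferSlot merges matching stacks or swaps slots between inventories, then notifies both.
; Equipping adds a weapon component to the owner if missing; Tick prints occupied slot indices.
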(event Custom|UpdateInventory
  (Default|CallOnInventoryUpdated))

(event Input|EnhancedActionEvents|EnhancedInputActionIA_WeaponSlot
  (params (ActionValue :type Boolean) (ElapsedSeconds :type Float%20%28double-precision%29) (TriggeredSeconds :type Float%20%28double-precision%29) (InputAction :type Input%20Action%20Object%20Reference :default "/Game/SKVOT/Inputs/Actions/IA_WeaponSlot.IA_WeaponSlot"))
  (CallFunction|EquipWeaponSlot))

(event EventBeginPlay
  (Utilities|Array|Resize (Variables|Default|GetItems) (Variables|Default|GetInventorySize)))

(event EventTick
  (params (DeltaSeconds :type Float%20%28single-precision%29))
  (for (_array_element _array_index) (Variables|Default|GetItems)
    (if (!= (.ItemID (Utilities|Struct|BreakS_ItemSlot _array_element)) "")
      (Development|PrintString (Utilities|String|ToString(Integer) _array_index) true true "(R=0.000000,G=0.660000,B=1.000000,A=1.000000)" 0.0))))

(fn AddItemtoInventory
  (params (Item :type BP%20Interactable%20Item%20Object%20Reference))
  (bind (_slotavailable _index) (CallFunction|AnySlotAvailable))
  (bind _output_get (LocalVariables|SetItemData (Actor|GetComponentbyClass Item "/Game/SKVOT/Blueprints/ActorComponents/AC_ItemData.AC_ItemData_C")))
  (while (and (> (Variables|/Game/SKVOT/Blueprints/ActorComponents/AC_ItemData.AC_ItemData_C|GetItemQuantity _output_get) 0) (not (LocalVariables|GetIsFull)))
    (bind (_array_index _slotavailable_2) (CallFunction|FindSlot (.rowname (Variables|/Game/SKVOT/Blueprints/ActorComponents/AC_ItemData.AC_ItemData_C|GetItemId (LocalVariables|GetItemData)))))
    (if _slotavailable_2
      (CallFunction|AddtoStack _array_index 1)
      (Math|Integer|DecrementInt (Variables|/Game/SKVOT/Blueprints/ActorComponents/AC_ItemData.AC_ItemData_C|GetItemQuantity (LocalVariables|GetItemData))
        (:%20%20
          (return true 0)))
      (elif _slotavailable
        (CallFunction|CreateNewStack (.rowname (Variables|/Game/SKVOT/Blueprints/ActorComponents/AC_ItemData.AC_ItemData_C|GetItemId (LocalVariables|GetItemData))) 1 _index)
        (Math|Integer|DecrementInt (Variables|/Game/SKVOT/Blueprints/ActorComponents/AC_ItemData.AC_ItemData_C|GetItemQuantity (LocalVariables|GetItemData))
          (:%20%20
            (return true 0)))
        (else
          (LocalVariables|SetIsFull true)))))
  (return (not (LocalVariables|GetIsFull)) (Variables|/Game/SKVOT/Blueprints/ActorComponents/AC_ItemData.AC_ItemData_C|GetItemQuantity (LocalVariables|GetItemData))))

(fn FindSlot
  (params (ItemId :type Name))
  (for (_array_element _array_index) (Variables|Default|GetItems)
    (if (and (== ItemId (.ItemID (Utilities|Struct|BreakS_ItemSlot _array_element))) (< (.ItemQuantity (Utilities|Struct|BreakS_ItemSlot _array_element)) (CallFunction|GetMaxStackSize ItemId)))
      (return _array_index true)))
  (return -1 false))

(fn GetMaxStackSize
  (params (ItemID :type Name))
  (bind _returnvalue (Utilities|GetDataTableRow "/Game/SKVOT/Structures/DT_ItemData.DT_ItemData" ItemID)
    (:then
      (return (Utilities|Struct|BreakS_ItemData _returnvalue)))))

(fn AddtoStack
  (params (Index :type Integer) (ItemQuantity :type Integer))
  (bind _items (Variables|Default|GetItems))
  (bind _output (Utilities|Array|Get(acopy) _items Index))
  (Utilities|Array|SetArrayElem (Variables|Default|GetItems) ItemQuantity (Utilities|Struct|MakeS_ItemSlot (.itemid _output) (+ (.itemquantity _output) ItemQuantity))))

(fn AnySlotAvailable
  (for (_array_element _array_index) (Variables|Default|GetItems)
    (if (== (.ItemQuantity (Utilities|Struct|BreakS_ItemSlot _array_element)) 0)
      (return true _array_index)))
  (return false -1))

(fn CreateNewStack
  (params (ItemId :type Name) (ItemQuantity :type Integer) (Index :type Integer))
  (Utilities|Array|SetArrayElem (Variables|Default|GetItems) Index (Utilities|Struct|MakeS_ItemSlot ItemId ItemQuantity)))

(fn TransferSlot
  (params (Index :type Integer) (SourceIndex :type Integer) (SourceInventory :type AC%20Inventory%20Component%20Object%20Reference))
  (bind _items (Variables|Default|GetItems))
  (bind _output (Utilities|Array|Get(acopy) _items Index))
  (Utilities|FlowControl|Sequence
    (:then_0
      (LocalVariables|SetSourceSlot (Utilities|Array|Get(acopy) (Variables|AC_InventoryComponent_C|GetItems SourceInventory) SourceIndex))
      (if (== (.ItemID (Utilities|Struct|BreakS_ItemSlot (LocalVariables|GetSourceSlot))) (.ItemID (Utilities|Struct|BreakS_ItemSlot (Utilities|Array|Get(acopy) (Variables|Default|GetItems) Index))))
        (CallFunction|CreateNewStack SourceInventory (select (> (Math|Integer|Clamp(Integer) (- (+ (.ItemQuantity (Utilities|Struct|BreakS_ItemSlot (LocalVariables|GetSourceSlot))) (.ItemQuantity (Utilities|Struct|BreakS_ItemSlot (Utilities|Array|Get(acopy) (Variables|Default|GetItems) Index)))) (CallFunction|GetMaxStackSize (.ItemID (Utilities|Struct|BreakS_ItemSlot (LocalVariables|GetSourceSlot))))) 0 (CallFunction|GetMaxStackSize (.ItemID (Utilities|Struct|BreakS_ItemSlot (LocalVariables|GetSourceSlot))))) 0) (.ItemID (Utilities|Struct|BreakS_ItemSlot (LocalVariables|GetSourceSlot))) "None") (Math|Integer|Clamp(Integer) (- (+ (.ItemQuantity (Utilities|Struct|BreakS_ItemSlot (LocalVariables|GetSourceSlot))) (.ItemQuantity (Utilities|Struct|BreakS_ItemSlot (Utilities|Array|Get(acopy) (Variables|Default|GetItems) Index)))) (CallFunction|GetMaxStackSize (.ItemID (Utilities|Struct|BreakS_ItemSlot (LocalVariables|GetSourceSlot))))) 0 (CallFunction|GetMaxStackSize (.ItemID (Utilities|Struct|BreakS_ItemSlot (LocalVariables|GetSourceSlot))))) SourceIndex)
        (CallFunction|CreateNewStack (Utilities|Struct|BreakS_ItemSlot (LocalVariables|GetSourceSlot)) (Math|Integer|Clamp(Integer) (+ (.ItemQuantity (Utilities|Struct|BreakS_ItemSlot (LocalVariables|GetSourceSlot))) (.ItemQuantity (Utilities|Struct|BreakS_ItemSlot (Utilities|Array|Get(acopy) (Variables|Default|GetItems) Index)))) 0 (CallFunction|GetMaxStackSize (.ItemID (Utilities|Struct|BreakS_ItemSlot (LocalVariables|GetSourceSlot))))) Index)
        (else
          (CallFunction|CreateNewStack SourceInventory (.itemid _output) (.itemquantity _output) SourceIndex)
          (CallFunction|CreateNewStack (.ItemID (Utilities|Struct|BreakS_ItemSlot (LocalVariables|GetSourceSlot))) (.ItemQuantity (Utilities|Struct|BreakS_ItemSlot (LocalVariables|GetSourceSlot))) Index))))
    (:then_1
      (CallFunction|UpdateInventory)
      (CallFunction|UpdateInventory SourceInventory))))

(fn EquipWeaponSlot
  (bind _returnvalue (Components|GetOwner))
  (if (== (.ItemID (Utilities|Struct|BreakS_ItemSlot (Utilities|Array|Get(acopy) (Variables|Default|GetItems)))) "0001A3")
    (if (Utilities|DoesObjectImplementInterface _returnvalue "/Game/SKVOT/Blueprints/Interfaces/BPI_WeaponOwner.BPI_WeaponOwner_C")
      (bind _output_get (LocalVariables|SetL_WeaponComponent (Actor|GetComponentbyClass _returnvalue "/Game/SKVOT/Blueprints/ActorComponents/AC_WeaponComponent.AC_WeaponComponent_C")))
      (Utilities|IsValid _output_get
        (:Is%20Valid
          _)
        (:Is%20Not%20Valid
          (bind _returnvalue_2 (Game|AddComponentbyClass (Components|GetOwner) "/Game/SKVOT/Blueprints/ActorComponents/AC_WeaponComponent.AC_WeaponComponent_C"))
          (bind _output_get_2 (LocalVariables|SetL_WeaponComponent _returnvalue_2))
          (Utilities|IsValid _output_get_2
            (:Is%20Valid
              _))))
      (Default|EquipWeapon (LocalVariables|GetL_WeaponComponent) "/Game/SKVOT/Blueprints/Items/Weapons/BP_BasicRevolver.BP_BasicRevolver_C"))))